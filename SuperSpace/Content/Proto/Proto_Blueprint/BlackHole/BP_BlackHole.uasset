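; BP_BlackHole is a moving black hole that stops beyond DistanceMax, pulls in physics objects, then destroys itself 1.5 seconds later.
; Once it is past that distance, Tick calls ApplyForce, pulling simulating components in GravitynfluanceRange toward the center with linear distance falloff and boosted vertical force.
; KillZone destroys overlapping physics actors and passes their mass to MassGained, which grows the Sphere through a timeline.
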(event `self.ReceiveBeginPlay`
  (set `self.startLocation` (`self.K2_GetActorLocation`))
  (set `self.HasStopped` false))

(event `self.ReceiveTick`
  (params (DeltaSeconds :type "Float (single-precision)"))
  (if (> (`KismetMathLibrary.Vector_Distance` (`self.K2_GetActorLocation`) (`self.startLocation`)) (`self.DistanceMax`))
    (`MovementComponent.StopMovementImmediately` (`self.BlackHole`))
    (set `self.HasStopped` true)
    (`self.ApplyForce`)
    (`KismetSystemLibrary.Delay` 1.5)
    (`self.K2_DestroyActor`)))

(event `self.KillZone.OnComponentBeginOverlap`
  (params (OverlappedComponent :type "PrimitiveComponent Object Reference") (OtherActor :type "Actor Object Reference") (OtherComp :type "PrimitiveComponent Object Reference") (OtherBodyIndex :type Integer) (bFromSweep :type Boolean) (SweepResult :type "HitResult Structure (by ref)"))
  (if (`SceneComponent.IsSimulatingPhysics` OtherComp "None")
    (`self.MassGained` (`PrimitiveComponent.GetMass` OtherComp))
    (`/Engine/EditorBlueprintResources/StandardMacros.IsValid` OtherActor
      (:`Is Valid`
        (`self.K2_DestroyActor` OtherActor)))))

(event `MassGained`
  (params (Mass :type "Float (double-precision)"))
  (set `self.CurrentScale` (`SceneComponent.K2_GetComponentScale` (`self.Sphere`)))
  (set `self.NewScale` (+ (`self.CurrentScale`) (* Mass (`self.GrowthRate`))))
  (bind (_direction _alpha) (`Timeline|Timeline` :!via `PlayFromStart`)
    (:`Update`
      (`SceneComponent.SetWorldScale3D` (`self.Sphere`) (`|EaseFunction` "Linear" _alpha (`self.CurrentScale`) (`self.NewScale`))))))

(fn `ApplyForce`
  (bind _returnvalue (`self.K2_GetActorLocation`))
  (for _array_element (`PrimitiveComponent.GetOverlappingComponents` (`self.GravitynfluanceRange`))
    (if (`SceneComponent.IsSimulatingPhysics` _array_element "None")
      (bind _returnvalue_2 (`SceneComponent.K2_GetComponentLocation` _array_element))
      (`PrimitiveComponent.AddForce` _array_element (* (`KismetMathLibrary.GetDirectionUnitVector` _returnvalue_2 _returnvalue) (* (- 1.0 (`KismetMathLibrary.FClamp` (/ (`KismetMathLibrary.Vector_Distance` _returnvalue _returnvalue_2) 5000.0))) 1000.0) (1.0 1.0 10.0) (`self.GravityStrength`)) "None" true))))

(fn `UserConstructionScript`)