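; Player-controlled prototype spaceship that advances along world Y, steers in X/Z with the mouse and fires black holes.
; Mouse input applies forward and lateral offsets, while Tick computes speed and pins the ship inside hardcoded X/Z bounds.
; Q and D play reversible timelines that tilt pitch 45 degrees either way.
; Left click spawns BP_BlackHole, gated by DoOnce and a cooldown timer shown on the game mode's DistanceUI.
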(event `Key|Q`
  (params (Key :type "Key Structure"))
  ;[1 1 1] Tangage
  (:`Pressed`
    (if (`self.keyTurn?`)
      (bind _output_get (set `self.StartRotation` (struct)))
      (set `self.TargetRotation` (`KismetMathLibrary.MakeRotator` (.roll _output_get) (+ (.pitch _output_get) -45.0) (.yaw _output_get)))
      (bind (_direction _smoothrotation) (`Timeline|SmoothRotation` :!via `PlayFromStart` :!label _label)
        (:`Update`
          (set `self.keyTurn?` false)
          (`self.K2_SetActorRelativeRotation` (`|EaseFunction` "Linear" _smoothrotation (`self.StartRotation`) (`self.TargetRotation`))))
        (:`Finished`
          (set `self.keyTurn?` true)))))
  (:`Released`
    (goto _label :!via `Reverse`)))

(event `Key|D`
  (params (Key :type "Key Structure"))
  ;[1 1 1] Tangage
  (:`Pressed`
    (if (`self.keyTurn?`)
      (bind _output_get (set `self.StartRotation` (struct)))
      (set `self.TargetRotation` (`KismetMathLibrary.MakeRotator` (.roll _output_get) (- (.pitch _output_get) -45.0) (.yaw _output_get)))
      (bind (_direction _smoothrotation) (`Timeline|Timeline` :!via `PlayFromStart` :!label _label_2)
        (:`Update`
          (set `self.keyTurn?` false)
          (`self.K2_SetActorRelativeRotation` (`|EaseFunction` "Linear" _smoothrotation (`self.StartRotation`) (`self.TargetRotation`))))
        (:`Finished`
          (set `self.keyTurn?` true)))))
  (:`Released`
    (goto _label_2 :!via `Reverse`)))

(event `self.ReceiveTick`
  (params (DeltaSeconds :type "Float (single-precision)"))
  (bind (_returnvalue_x _returnvalue_y _returnvalue_z) (`KismetMathLibrary.BreakVector` (`self.K2_GetActorLocation`)))
  (bind _locatio_x (`self.Locatio_X`))
  (bind _location_z (`self.Location_Z`))
  ;[0.3605 0 1] Mouvement of ship
  (`|ExecutionSequence`
    (:`then_0`
      (`GameUserSettings.GetGameUserSettings`)
      (set `self.Locatio_X` _returnvalue_x)
      (set `self.Location_Y` _returnvalue_y)
      (set `self.Location_Z` _returnvalue_z)
      (set `self.ShipSpeed` (* (`self.BaseSpeed`) (`self.SpeedMultiplier`)))
      (set `self.NewLocation_Y` (+ (`self.Location_Y`) (.x (* (* (`self.GetActorForwardVector`) 1200.0) DeltaSeconds))))
      (switch `int` (+ (* (`KismetMathLibrary.Conv_BoolToInt` (<= _locatio_x 70.0)) 1) (* (`KismetMathLibrary.Conv_BoolToInt` (>= _locatio_x 2890.0)) 2) (* (`KismetMathLibrary.Conv_BoolToInt` (<= _location_z 440.0)) 3) (* (`KismetMathLibrary.Conv_BoolToInt` (>= _location_z 2110.0)) 4))
        (:`1`
          (`self.K2_SetActorLocation` (`KismetMathLibrary.MakeVector` 71.0 (`self.NewLocation_Y`) (`self.Location_Z`))))
        (:`2`
          (`self.K2_SetActorLocation` (`KismetMathLibrary.MakeVector` 2889.0 (`self.NewLocation_Y`) (`self.Location_Z`))))
        (:`3`
          (`self.K2_SetActorLocation` (`KismetMathLibrary.MakeVector` (`self.Locatio_X`) (`self.NewLocation_Y`) 441.0)))
        (:`4`
          (`self.K2_SetActorLocation` (`KismetMathLibrary.MakeVector` (`self.Locatio_X`) (`self.NewLocation_Y`) 2109.0))))
      (set `self.ShipSpeed` 0.0))
    (:`then_1`
      (if (`KismetSystemLibrary.K2_IsValidTimerHandle` (`self.CoolDownTimer`))
        (`ProgressBar.SetPercent` (`/Game/Proto/Interface/Score_UI.ProgressBar_0` (`self.Distance UI`)) (/ (`KismetSystemLibrary.K2_GetTimerElapsedTimeHandle` (`self.CoolDownTimer`)) (`self.CoolDown`)))))))

(event `InputVectorAxis|Mouse2D`
  (params (AxisValue :type "Vector Structure"))
  (bind _shipspeed (`self.ShipSpeed`))
  ;[0.3605 0 1] Mouvement of ship
  (`self.K2_AddActorWorldOffset` (`KismetMathLibrary.MakeVector` (* (* AxisValue_X _shipspeed) -10.0) (.x (* (* (`self.GetActorForwardVector`) 1200.0) (stale `self.ReceiveTick` DeltaSeconds))) (* (* AxisValue_Y _shipspeed) 20.0))))

(event `self.ReceiveBeginPlay`
  (bind _asbp_third_person_game_mode (cast `/Game/ThirdPerson/Blueprints/BP_ThirdPersonGameMode` (`GameplayStatics.GetGameMode`)))
  (set `self.Distance UI` (`/Game/ThirdPerson/Blueprints/BP_ThirdPersonGameMode.DistanceUI` _asbp_third_person_game_mode)))

(event `Key|LeftMouseButton`
  (params (Key :type "Key Structure"))
  ;[1 1 1] commande de tire
  (:`Pressed`
    (`/Engine/EditorBlueprintResources/StandardMacros.DoOnce` false :!label _label_3
      (:`Completed`
        (`|SpawnActorFromClass` "/Game/Proto/Proto_Blueprint/BlackHole/BP_BlackHole.BP_BlackHole_C" (`SceneComponent.K2_GetComponentToWorld` (`self.ProjectileSpawnPosition`)) "AlwaysSpawn" "MultiplyWithRoot" null null)
        (`ProgressBar.SetPercent` (`/Game/Proto/Interface/Score_UI.ProgressBar_0` (`self.Distance UI`)) 0.0)
        (bind _returnvalue (`KismetSystemLibrary.K2_SetTimerDelegate` (delegate `FinishCooldown`) (`self.CoolDown`)))
        (set `self.CoolDownTimer` _returnvalue)))))

(event `FinishCooldown`
  ;[1 1 1] commande de tire
  (`KismetSystemLibrary.K2_ClearAndInvalidateTimerHandle` (`self.CoolDownTimer`))
  (goto _label_3 :!via `Reset`))

(fn `UserConstructionScript`)