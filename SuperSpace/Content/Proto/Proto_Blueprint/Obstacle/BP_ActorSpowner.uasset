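; BP_ActorSpowner is a prototype obstacle spawner that spawns actors, named as asteroids, while a player is inside its trigger.
; Overlap by an actor tagged Player prints a debug string and starts a fast looping timer, which is cleared when that actor leaves.
; Each timer tick spawns an actor at a random point within the spawn trigger's box extent; the spawned class is not set in the visible graph.
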(event `StopSpawningActors`
  (`KismetSystemLibrary.K2_ClearAndInvalidateTimerHandle` (stale `self.SpawnAsteroide_Trigger.OnComponentBeginOverlap` _returnvalue)))

(event `self.SpawnAsteroide_Trigger.OnComponentBeginOverlap`
  (params (OverlappedComponent :type "PrimitiveComponent Object Reference") (OtherActor :type "Actor Object Reference") (OtherComp :type "PrimitiveComponent Object Reference") (OtherBodyIndex :type Integer) (bFromSweep :type Boolean) (SweepResult :type "HitResult Structure (by ref)"))
  (if (`self.ActorHasTag` OtherActor "Player")
    (`KismetSystemLibrary.PrintString` "Hello")
    (bind _returnvalue (`KismetSystemLibrary.K2_SetTimerDelegate` (delegate `EventAsteroide`) 0.15 true))))

(event `EventAsteroide`
  (bind _spawnasteroide_trigger (`self.SpawnAsteroide_Trigger`))
  (`|SpawnActorFromClass` "/Game/Proto/Proto_Blueprint/Obstacle/BP_Asteroide.BP_Asteroide_C" (`KismetMathLibrary.MakeTransform` (`KismetMathLibrary.RandomPointInBoundingBox` (`SceneComponent.K2_GetComponentLocation` _spawnasteroide_trigger) (`BoxComponent.BoxExtent` _spawnasteroide_trigger))) "Undefined" "MultiplyWithRoot" null null))

(event `self.SpawnAsteroide_Trigger.OnComponentEndOverlap`
  (params (OverlappedComponent :type "PrimitiveComponent Object Reference") (OtherActor :type "Actor Object Reference") (OtherComp :type "PrimitiveComponent Object Reference") (OtherBodyIndex :type Integer))
  (if (`self.ActorHasTag` OtherActor "Player")
    (`self.StopSpawningActors`)))

(fn `UserConstructionScript`)